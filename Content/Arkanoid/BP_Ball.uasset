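; BP_Ball is the Arkanoid ball, which moves itself, breaks blocks and keeps the score.
; Each Tick it does a swept world offset along Direction at Speed and reflects Direction off the surface normal on a blocking hit.
; Hit actors tagged "Block" are destroyed and trigger AddPoints, which updates the W_Score widget created and added to the viewport at BeginPlay.
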(event `self.ReceiveBeginPlay`
  (bind _returnvalue (`|CreateWidget` "/Game/Arkanoid/W_Score.W_Score_C"))
  (bind _output_get (set `self.ScoreWidget` _returnvalue))
  (`UserWidget.AddToViewport` _output_get 0))

(event `self.ReceiveTick`
  (params (DeltaSeconds :type "Float (single-precision)"))
  ;[1 1 1] Sweep блокирует шар в стее
  (bind _sweephitresult (`self.K2_AddActorWorldOffset` (* DeltaSeconds (* (`self.Speed`) (`self.Direction`))) true))
  (bind (_bblockinghit _binitialoverlap _time _distance _location _impactpoint _normal _impactnormal _physmat _hitactor) (`GameplayStatics.BreakHitResult` _sweephitresult))
  (if _bblockinghit
    (set `self.Direction` (`KismetMathLibrary.GetReflectionVector` (`self.Direction`) _normal))
    (if (`self.ActorHasTag` _hitactor "Block")
      (`self.K2_DestroyActor` _hitactor)
      (`self.AddPoints` 1))))

(event `AddPoints`
  (params (Points :type Integer))
  (set `self.Points` (+ Points (`self.Points`)))
  (`/Game/Arkanoid/W_Score.UpdateScore` (`self.ScoreWidget`) (`self.Points`)))

(fn `UserConstructionScript`)